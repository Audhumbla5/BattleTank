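; Tank player controller that reads serial data from an Arduino and prints it, without yet driving the tank.
; BeginPlay opens and flushes the COM port, and EndPlay closes it.
; Tick polls bytes for a two-byte header (182, then 147), then calls ReadWheelAndTele.
; That function copies the following payload bytes into an array from index 2, which Tick concatenates into a debug string.
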(event EventBeginPlay
  (bind (_bopened _returnvalue) (Class|Serial|OpenComPort 1 9600))
  (if _bopened
    (bind _output_get (Variables|Default|SetArduino _returnvalue))
    (Class|Serial|Flush _output_get)
    (Development|PrintString "Port opened")
    (else
      (Development|PrintString "Port not opened"))))

(event EventTick
  (params (DeltaSeconds :type Float%20%28single-precision%29))
  (bind _arduino (Variables|Default|GetArduino))
  (Variables|Default|Setmessage "\"\"")
  (Utilities|IsValid _arduino
    (:Is%20Valid
      (bind (_bsuccess _returnvalue) (Class|Serial|ReadByte _arduino))
      (if _bsuccess
        (if (== (Math|Conversions|ToInteger(Byte) _returnvalue) 182)
          (bind _output_get (Variables|Default|SetinByte (Math|Conversions|ToInteger(Byte) _returnvalue)))
          (Variables|Default|Setmessage (Utilities|String|Append (Variables|Default|Getmessage) " " (Utilities|String|ToString(Integer) _output_get)))
          (bind _returnvalue_2 (Class|Serial|ReadByte _arduino))
          (Variables|Default|Setmessage "")
          (switch string (Utilities|String|ToString(Byte) _returnvalue_2)
            (:147
              (bind _wheeltelearray (CallFunction|ReadWheelandTele (Variables|Default|GetArduino)))
              (for _array_element _wheeltelearray
                (Variables|Default|Setmessage (Utilities|String|Append (Variables|Default|Getmessage) " " (Utilities|String|ToString(Integer) _array_element))))
              (Development|PrintString (Variables|Default|Getmessage)))))))))

(event MouseInput|EventActorOnClicked
  (params (ButtonPressed :type Key%20Structure)))

(event EventEndPlay
  (params (EndPlayReason :type EEndPlayReason%20Enum :default "Destroyed"))
  (bind _arduino (Variables|Default|GetArduino))
  (Utilities|IsValid _arduino
    (:Is%20Valid
      (Class|Serial|Close _arduino))))

(fn ConstructionScript)

(fn ReadWheelandTele
  (params (SerialIn :type Serial%20Object%20Reference))
  (bind _returnvalue (Class|Serial|ReadByte SerialIn))
  (LocalVariables|SetinValue (Math|Conversions|ToInteger(Byte) _returnvalue))
  (for _index (range 2 22)
    (Utilities|Array|SetArrayElem (LocalVariables|GetmessageArray) _index (LocalVariables|GetinValue))
    (bind _returnvalue_2 (Class|Serial|ReadByte SerialIn))
    (LocalVariables|SetinValue (Math|Conversions|ToInteger(Byte) _returnvalue_2)))
  (return (LocalVariables|GetmessageArray)))